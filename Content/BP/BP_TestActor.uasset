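; Test actor that tries out downloading and unzipping remote content at runtime.
; On BeginPlay, an async DownloadAndUnzipContent node fetches a zip from a hard-coded Azure Blob SAS URL and targets a fixed local project Content folder, printing progress and completion.
; Disconnected experiments remain for HTTP requests, RuntimeArchiver extraction, and async asset loading onto a skeletal mesh component; none of them run.
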(event `CustomEvent_0`
  (params (bSuccess :type Boolean)))

(event `self.ReceiveBeginPlay`
  (bind _bsuccess (`Async_HTTP_Request.DownloadAndUnzipContent` (make `HttpRequestData` "GET" "https://vcconfigurator.blob.core.windows.net/models/001.zip?sp=r&st=2023-06-14T09:59:24Z&se=2024-06-14T17:59:24Z&spr=https&sv=2022-11-02&sr=b&sig=UDi%2FWDPYvkNO4ZmYKQbA66yJQkzrmizedT6Jf5WQhd4%3D") (make `UnzipData` "/Script/RuntimeArchiver.RuntimeArchiverZip") (make `Directory` "E:/Ashot/Files/Unreal engine/HTTP_request/Content/test" "cookies/001.zip" "" true))
    (:`then`
      (`KismetSystemLibrary.PrintString` "Hello"))
    (:`OnRequestCompleted`
      (`KismetSystemLibrary.PrintString` (`KismetStringLibrary.Conv_BoolToString` _bsuccess) true true (struct :`R` 1.0 :`B` 0.076087 :`A` 1.0)))
    (:`OnRequestProgress`
      (`KismetSystemLibrary.PrintString` "Hello" true true (struct :`G` 0.111714 :`B` 1.0 :`A` 1.0) 0.1))))

(fn `UserConstructionScript`)